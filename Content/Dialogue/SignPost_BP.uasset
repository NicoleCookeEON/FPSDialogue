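; Signpost actor that shows a text message on screen when interacted with.
; Interact, from the Interact_I interface, toggles a DialogueWidget: it creates the widget for player 0 and passes in the per-instance MyText, or removes and clears an existing one.
; When a FirstPersonCharacter leaves the Box volume, the widget is removed and its reference cleared, without a validity check.
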(event OnComponentEndOverlap(Box)
  (params (OverlappedComponent :type Primitive%20Component%20Object%20Reference) (OtherActor :type Actor%20Object%20Reference) (OtherComp :type Primitive%20Component%20Object%20Reference) (OtherBodyIndex :type Integer))
  ;[1 1 1] Removes the text displayed on screen once far enough from the actor
  (Utilities|Casting|CastToFirstPersonCharacter OtherActor)
  ;;[1 1 1] This removes the widget
  (Widget|RemovefromParent (Variables|Default|GetDialogueWidget))
  ;;[1 1 1] Not choosing a drop down will make this empty/blank/void/null
  (Variables|Default|SetDialogueWidget 0))

(event Collision|EventActorBeginOverlap
  (params (OtherActor :type Actor%20Object%20Reference)))

(event EventTick
  (params (DeltaSeconds :type Float%20%28single-precision%29)))

(event EventInteract
  ;[1 1 1] This has been added from the Interact interaface (Interact_I) - In class settings
  ;;[1 1 1] This checks if the dialogue widget exsists
  (Utilities|IsValid (Variables|Default|GetDialogueWidget)
    (:Is%20Valid
      ;;[1 1 1] This removes the widget
      (Widget|RemovefromParent (Variables|Default|GetDialogueWidget))
      ;;[1 1 1] Not choosing a drop down will make this empty/blank/void/null
      (Variables|Default|SetDialogueWidget 0))
    (:Is%20Not%20Valid
      ;;[1 1 1] Attaching the widget to the current player
      (bind _returnvalue (UserInterface|CreateWidget "/Game/Dialogue/DialogueWidget.DialogueWidget_C" (Game|GetPlayerController 0)))
      ;;[1 1 1] This was promoted to save a refference to dialouge widget
      (bind _output_get (Variables|Default|SetDialogueWidget _returnvalue))
      ;;[1 1 1] Just adds this to the current players viewport
      (UserInterface|Viewport|AddtoViewport _output_get 0)
      ;;[1 1 1] This get the text created and binded (DialogueText). Also make the text editable on the acotor asigned.
      (Variables|/Game/Dialogue/DialogueWidget.DialogueWidget_C|SetDialogueText (Variables|Default|GetDialogueWidget) (Variables|Default|GetMyText)))))

(fn ConstructionScript)