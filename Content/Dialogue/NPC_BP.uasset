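; NPC Blueprint that shows data-table-driven dialogue lines when interacted with and turns to face the player.
; On BeginPlay it caches Dialogue table row names matching its NPCID.
; Each Interact advances LineCurrent, creates or reuses the dialogue widget, and shows the line matching ConversationID and LineID.
; The widget is removed when FirstPersonCharacter leaves the Box, or when no single line matches, which also resets the line counter.
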(event OnComponentEndOverlap(Box)
  (params (OverlappedComponent :type Primitive%20Component%20Object%20Reference) (OtherActor :type Actor%20Object%20Reference) (OtherComp :type Primitive%20Component%20Object%20Reference) (OtherBodyIndex :type Integer))
  ;[1 1 1] Comment
  (Utilities|Casting|CastToFirstPersonCharacter OtherActor)
  ;;[1 1 1] This removes the widget
  (Widget|RemovefromParent (Variables|Default|GetDialogueWidget))
  ;;[1 1 1] Not choosing a drop down will make this empty/blank/void/null
  (Variables|Default|SetDialogueWidget 0))

(event EventBeginPlay
  ;[1 1 1] Looking for the NPC and looking which one the ID belongs to it
  ;[1 1 1] This gets an array of the NPCs
  (bind _outrownames (DataTable|GetDataTableRowNames "/Game/Dialogue/Dialogue.Dialogue"))
  ;[1 1 1] Go through every single row, break that row down, look for the NPC ID. If matches record the row name that belongs to that NPC.
  (for _array_element _outrownames
    (bind _returnvalue (Utilities|GetDataTableRow "/Game/Dialogue/Dialogue.Dialogue" _array_element)
      (:then
        ;[1 1 1] If NPC ID is the same then we want to record is the row name
        (if (== (.NPC_ID (Utilities|Struct|BreakDialogueStructure _returnvalue)) (Variables|Default|GetNPC_ID))
          ;[1 1 1] Adds the array of names
          (Utilities|Array|Add (Variables|Default|GetMyDialogue) _array_element))))))

(event EventInteract
  ;[1 1 1] Function Interact_I - Increase the current line we are on and then create a dialogue window
  ;[1 1 1] Line current is currently 1 this will now increase by 1. Interact again the number will increase.
  (Math|Integer|IncrementInt (Variables|Default|GetLineCurrent)
    (:%20%20
      ;[1 1 1] Create the widgets
      (CallFunction|DialogueCreate)
      ;[1 1 1] This gets the charater to turn on the z axis when interated with
      (Transformation|SetActorRotation (Math|Rotator|MakeRotator 0.0 0.0 (.Yaw (Math|Rotator|BreakRotator (Math|Rotator|FindLookatRotation (Transformation|GetActorLocation) (Transformation|GetActorLocation (Game|GetPlayerCharacter 0))))))))))

(fn ConstructionScript)

(fn DialogueCreate
  ;[1 1 1] Is dialogue already open?
  (Utilities|IsValid (Variables|Default|GetDialogueWidget)
    (:Is%20Valid
      ;[1 1 1] New function to create text
      (bind _returnline (CallFunction|DialogueGetLine))
      ;[1 1 1] This is from DialogueWdget binded on the text
      (Variables|/Game/Dialogue/DialogueWidget.DialogueWidget_C|SetDialogueText (Variables|Default|GetDialogueWidget) _returnline))
    (:Is%20Not%20Valid
      ;[1 1 1] Create new widget, display this on screen and then change the text to be a perticular line of dialogue
      (bind _returnvalue (UserInterface|CreateWidget "/Game/Dialogue/DialogueWidget.DialogueWidget_C" (Game|GetPlayerController 0)))
      (bind _output_get (Variables|Default|SetDialogueWidget _returnvalue))
      (UserInterface|Viewport|AddtoViewport _output_get 0)
      ;[1 1 1] New function to create text
      (bind _returnline_2 (CallFunction|DialogueGetLine))
      ;[1 1 1] This is from DialogueWdget binded on the text
      (Variables|/Game/Dialogue/DialogueWidget.DialogueWidget_C|SetDialogueText (Variables|Default|GetDialogueWidget) _returnline_2))))

(fn DialogueGetLine
  ;[1 1 1] This is going to check for all the rows names
  (for _array_element (Variables|Default|GetMyDialogue)
    (bind _returnvalue (Utilities|GetDataTableRow "/Game/Dialogue/Dialogue.Dialogue" _array_element)
      (:then
        ;[1 1 1] This saves the array of dialogue. This is to make sure we only have one line out.
        (if (and (== (.Conversation_ID (Utilities|Struct|BreakDialogueStructure _returnvalue)) (Variables|Default|GetConversation_ID)) (== (.Line_ID (Utilities|Struct|BreakDialogueStructure _returnvalue)) (Variables|Default|GetLineCurrent)))
          (Utilities|Array|Add (LocalVariables|GetReturnedLines) (.Dialogue (Utilities|Struct|BreakDialogueStructure _returnvalue)))))))
  (if (== (Utilities|Array|Length (LocalVariables|GetReturnedLines)) 1)
    ;[1 1 1] This completes us getting the row
    (return (Utilities|Array|Get(acopy) (LocalVariables|GetReturnedLines)))
    (else
      ;[1 1 1] This destroys the widget
      (Widget|RemovefromParent (Variables|Default|GetDialogueWidget))
      (Variables|Default|SetDialogueWidget 0)
      ;[1 1 1] This resets the row back to 0
      (Variables|Default|SetLineCurrent 0))))